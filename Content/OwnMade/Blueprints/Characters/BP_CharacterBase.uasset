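; Base character Blueprint that fires a projectile when the left mouse button is pressed.
; The input calls a server-named spawn event, which creates a BP_ProjectileBase at the mesh's ProjectileSpawnPoint socket, ignoring collisions.
; The event then adds a fixed-speed push along the camera's forward vector to the velocity of the projectile's movement component, so shots follow the camera's direction.
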(event Custom|Server_SpawnProjectile
  (bind _returnvalue (Game|SpawnActorfromClass "/Game/OwnMade/Blueprints/Actors/BP_ProjectileBase.BP_ProjectileBase_C" (Math|Transform|MakeTransform (Transformation|GetSocketLocation (Variables|Character|GetMesh) "ProjectileSpawnPoint") "0, 0, 0" "1,1,1") "AlwaysSpawn" 0 0))
  (Variables|/Script/Engine.MovementComponent|SetVelocity (Actor|GetComponentbyClass _returnvalue "/Script/Engine.ProjectileMovementComponent") (+ (Variables|/Script/Engine.MovementComponent|GetVelocity (Actor|GetComponentbyClass _returnvalue "/Script/Engine.ProjectileMovementComponent")) (* (Math|Vector|GetForwardVector (Variables|Default|GetCamera)) 2e+03))))

(event EventBeginPlay)

(event Collision|EventActorBeginOverlap
  (params (OtherActor :type Actor%20Object%20Reference)))

(event EventTick
  (params (DeltaSeconds :type Float%20%28single-precision%29)))

(event Input|MouseEvents|LeftMouseButton
  (params (Key :type Key%20Structure :default "None"))
  (:Pressed
    (CallFunction|ServerSpawnProjectile)))

(fn ConstructionScript)