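; Base actor for area-of-effect magic attacks that deals a one-shot burst of damage where it spawns.
; BeginPlay applies radial damage around the actor, credited to its owner through BP_DamageTypeBase, and draws a matching debug sphere.
; A Server_ApplyDamage event for damaging non-owner BP_CharacterBase targets exists but is unused, as the capsule overlap event is empty and its call is disconnected.
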(event OnComponentBeginOverlap(Capsule)
  (params (OverlappedComponent :type Primitive%20Component%20Object%20Reference) (OtherActor :type Actor%20Object%20Reference) (OtherComp :type Primitive%20Component%20Object%20Reference) (OtherBodyIndex :type Integer) (bFromSweep :type Boolean) (SweepResult :type Hit%20Result%20Structure%20%28by%20ref%29)))

(event Custom|Server_ApplyDamage
  (params (HittedActor :type Actor%20Object%20Reference))
  (bind _returnvalue (Components|GetOwner))
  (if (not (== HittedActor _returnvalue))
    (bind _asbp_character_base (Utilities|Casting|CastToBP_CharacterBase HittedActor))
    (Game|Damage|ApplyDamage _asbp_character_base 1e+01 0 _returnvalue "/Game/OwnMade/Blueprints/DamageTypes/BP_DamageTypeBase.BP_DamageTypeBase_C")))

(event EventBeginPlay
  (bind _returnvalue (Transformation|GetActorLocation))
  (Game|Damage|ApplyRadialDamage 25.0 _returnvalue 3e+02 "/Game/OwnMade/Blueprints/DamageTypes/BP_DamageTypeBase.BP_DamageTypeBase_C" 0 (Components|GetOwner) 0 false "ECC_Visibility")
  (Rendering|Debug|DrawDebugSphere _returnvalue 3e+02 12 "(R=1.000000,G=1.000000,B=1.000000,A=1.000000)" 1.0 5.0))

(event Collision|EventActorBeginOverlap
  (params (OtherActor :type Actor%20Object%20Reference)))

(event EventTick
  (params (DeltaSeconds :type Float%20%28single-precision%29)))

(fn ConstructionScript)